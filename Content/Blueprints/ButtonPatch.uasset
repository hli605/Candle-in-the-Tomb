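; ButtonPatch is a pressure button in an ordered puzzle that opens a door, with buttons safe for the male or female character.
; On overlap, an active button checks the character type and whether it is first in Level1Mechanics' SafeButtons list.
; A correct press deactivates it and removes it from the list, destroying the Door once the list empties.
; A wrong press briefly hides the button and disables its collision.
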(event `self.ReceiveBeginPlay`
  (bind _outactors (`GameplayStatics.GetAllActorsOfClass` "/Game/Blueprints/Level1Mechanics.Level1Mechanics_C"))
  (set `self.MyLevelInfo` (`|GetArrayItem` _outactors)))

(event `self.ReceiveActorBeginOverlap`
  (params (OtherActor :type "Actor Object Reference"))
  ;[1 1 1] Manage with player collision
  (if (`self.Activated`)
    (cast `/Game/Blueprints/MaleCharacter` OtherActor)
    (cast `/Game/Blueprints/FemaleCharacter` OtherActor
      (:`then`
        (if (`self.SafeForFemale`)
          (if (== (`|GetArrayItem` (`/Game/Blueprints/Level1Mechanics.SafeButtons` (`self.MyLevelInfo`))) self) :!label _label
            (set `self.Activated` false)
            (`KismetArrayLibrary.Array_Remove` (`/Game/Blueprints/Level1Mechanics.SafeButtons` (`self.MyLevelInfo`)))
            (if (== (`KismetArrayLibrary.Array_Length` (`/Game/Blueprints/Level1Mechanics.SafeButtons` (`self.MyLevelInfo`))) 0)
              (`self.K2_DestroyActor` (`self.Door`)))
            (else
              (`self.Disable` true :!label _label_2)
              (`KismetSystemLibrary.Delay` 2.0)
              (`self.Disable` false)))
          (else
            (goto _label_2))))
      (:`CastFailed`
        (if (`self.SafeForMale`)
          (goto _label)
          (else
            (goto _label_2)))))))

(event `Disable`
  (params (disable :type Boolean))
  ;[1 1 1] SetActive function in Unity
  (if disable
    (`self.SetActorHiddenInGame` true)
    (`self.SetActorEnableCollision` false)
    (else
      (`self.SetActorHiddenInGame` false)
      (`self.SetActorEnableCollision` true))))

(fn `UserConstructionScript`)