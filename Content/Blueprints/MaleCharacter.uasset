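; MaleCharacter is a playable character for a two-character game, with shared logic that also accounts for a FemaleCharacter variant.
; On BeginPlay it records its spawn transform and gender with CandleInTheTombMode.
; Overlapping a "Death"-tagged actor costs a life and respawns that character, or on game over respawns both players and resets lives.
; Its input axes drive world-aligned movement for itself and player character 1, the female.
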(event `self.ReceiveBeginPlay`
  (`|ExecutionSequence`
    (:`then_0`
      ;[1 1 1] Character Variables setup
      (bind _ascandle_in_the_tomb_mode (cast `/Game/Blueprints/CandleInTheTombMode` (`GameplayStatics.GetGameMode`)))
      (bind _output_get (set `self.GameMode` _ascandle_in_the_tomb_mode))
      (cast `/Game/Blueprints/FemaleCharacter` self
        (:`then`
          (set `/Game/Blueprints/CandleInTheTombMode.Female Spawn Transform` (`self.GetTransform`) _output_get)
          (set `self.isMale` false))
        (:`CastFailed`
          (set `/Game/Blueprints/CandleInTheTombMode.Male Spawn Transform` (`self.GetTransform`) _output_get)
          (set `self.isMale` true))))))

(event `self.ReceiveActorBeginOverlap`
  (params (OtherActor :type "Actor Object Reference"))
  (bind _gamemode (`self.GameMode`))
  ;[1 1 1] Death Trigger
  (if (`self.ActorHasTag` OtherActor "Death")
    (`/Game/Blueprints/CandleInTheTombMode.LoseLife` (`self.GameMode`))
    (if (`/Game/Blueprints/CandleInTheTombMode.GameOver` (`self.GameMode`))
      (bind _outactors (`GameplayStatics.GetAllActorsOfClass` "MaleCharacter_C"))
      (for _array_element _outactors
        (`self.K2_DestroyActor` _array_element))
      (`/Game/Blueprints/CandleInTheTombMode.RespawnPlayers` (`self.GameMode`))
      (set `/Game/Blueprints/CandleInTheTombMode.Lives` 3 (`self.GameMode`))
      (elif (`self.isMale`)
        (`/Game/Blueprints/CandleInTheTombMode.RespawnMaleChar` _gamemode)
        (`self.K2_DestroyActor`)
        (else
          (`/Game/Blueprints/CandleInTheTombMode.RespawnFemChar` _gamemode)
          (`self.K2_DestroyActor`))))))

(event `InputAxis|FemCharMoveUp`
  (params (AxisValue :type "Float (single-precision)"))
  ;[1 1 1] Female Character Movement
  (`self.AddMovementInput` (`GameplayStatics.GetPlayerCharacter` 1) (1.0 0.0 0.0) AxisValue false))

(event `InputAxis|MaleCharMoveUp`
  (params (AxisValue :type "Float (single-precision)"))
  ;[1 1 1] Male Character Movement
  (`self.AddMovementInput` (1.0 0.0 0.0) AxisValue))

(event `InputAxis|FemCharMoveRight`
  (params (AxisValue :type "Float (single-precision)"))
  ;[1 1 1] Female Character Movement
  (`self.AddMovementInput` (`GameplayStatics.GetPlayerCharacter` 1) (0.0 1.0 0.0) AxisValue false))

(event `InputAxis|MaleCharMoveRight`
  (params (AxisValue :type "Float (single-precision)"))
  ;[1 1 1] Male Character Movement
  (`self.AddMovementInput` (0.0 1.0 0.0) AxisValue))

(fn `UserConstructionScript`)