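; Game mode for Candle in the Tomb that handles respawning for two players and tracks a single Lives counter.
; Respawn events spawn the male and female characters at stored transforms, together or individually, and possess them with player controllers 0 and 1 respectively.
; LoseLife decrements and prints Lives, then sets the GameOver flag once none remain; nothing here calls these events or acts on that flag.
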(event `RespawnPlayers`
  ;[1 1 1] Character Respawn
  (bind _returnvalue (`|SpawnActorFromClass` "/Game/Blueprints/MaleCharacter.MaleCharacter_C" (`self.Male Spawn Transform`) "Undefined" "OverrideRootScale" null null))
  (`Controller.Possess` (`GameplayStatics.GetPlayerController` 0) _returnvalue)
  (bind _returnvalue_2 (`|SpawnActorFromClass` "/Game/Blueprints/FemaleCharacter.FemaleCharacter_C" (`self.Female Spawn Transform`) "Undefined" "OverrideRootScale" null null))
  (`Controller.Possess` (`GameplayStatics.GetPlayerController` 1) _returnvalue_2))

(event `RespawnMaleChar`
  ;[1 1 1] Character Respawn
  (bind _returnvalue (`|SpawnActorFromClass` "/Game/Blueprints/MaleCharacter.MaleCharacter_C" (`self.Male Spawn Transform`) "Undefined" "OverrideRootScale" null null))
  (`Controller.Possess` (`GameplayStatics.GetPlayerController` 0) _returnvalue))

(event `RespawnFemChar`
  ;[1 1 1] Character Respawn
  (bind _returnvalue (`|SpawnActorFromClass` "/Game/Blueprints/FemaleCharacter.FemaleCharacter_C" (`self.Female Spawn Transform`) "Undefined" "OverrideRootScale" null null))
  (`Controller.Possess` (`GameplayStatics.GetPlayerController` 1) _returnvalue))

(event `LoseLife`
  ;[1 1 1] Life control
  (bind _output_get (set `self.Lives` (- (`self.Lives`) 1)))
  (`KismetSystemLibrary.PrintString` (`KismetStringLibrary.Conv_IntToString` _output_get))
  (if (<= (`self.Lives`) 0)
    (set `self.GameOver` true)
    (else
      (set `self.GameOver` false))))

(fn `UserConstructionScript`)